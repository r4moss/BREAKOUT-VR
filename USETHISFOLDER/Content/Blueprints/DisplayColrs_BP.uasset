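; DisplayColrs_BP is an actor that displays a randomly generated three-color combination and stores its numeric equivalent.
; On BeginPlay it rolls three independent digits and uses each to pick a material from the Colors array for the Color1, Color2 and Color3 components.
; It packs the digits into Storage as a three-digit number, with Color1 as the hundreds digit and Color3 as the units.
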(event `self.ReceiveBeginPlay`
  (bind _output_get (set `self.Random1` (`KismetMathLibrary.RandomIntegerInRange` 0 9)))
  (bind _output_get_2 (set `self.Random2` (`KismetMathLibrary.RandomIntegerInRange` 0 9)))
  (bind _output_get_3 (set `self.Random3` (`KismetMathLibrary.RandomIntegerInRange` 0 9)))
  (`PrimitiveComponent.SetMaterial` (`self.Color1`) 0 (`|GetArrayItem` (`self.Colors`) (`self.Random1`)))
  (`PrimitiveComponent.SetMaterial` (`self.Color2`) 0 (`|GetArrayItem` (`self.Colors`) (`self.Random2`)))
  (`PrimitiveComponent.SetMaterial` (`self.Color3`) 0 (`|GetArrayItem` (`self.Colors`) (`self.Random3`)))
  (set `self.storage` (+ (* _output_get 100) (* _output_get_2 10) _output_get_3)))

(fn `UserConstructionScript`)