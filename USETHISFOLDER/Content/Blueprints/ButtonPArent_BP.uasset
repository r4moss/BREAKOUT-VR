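; Base Blueprint for a physical button that visually depresses when a VR pawn touches it.
; BeginPlay caches the button root's relative location as the rest position.
; Actor overlap with a VRPawn slides the root a short way along negative Y, and end overlap slides it back, both through MoveComponentTo.
; Tick also runs a delayed debug print of the actor's world location.
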(event `self.ReceiveBeginPlay`
  (set `self.ButtonStart` (`SceneComponent.RelativeLocation` (`self.ButtonRoot`))))

(event `self.ReceiveTick`
  (params (DeltaSeconds :type "Float (single-precision)"))
  (`KismetSystemLibrary.Delay` 5.0)
  (`KismetSystemLibrary.PrintString` (`KismetStringLibrary.Conv_VectorToString` (`self.K2_GetActorLocation`))))

(event `self.ReceiveActorBeginOverlap`
  (params (OtherActor :type "Actor Object Reference"))
  (cast `/Game/VRTemplate/Blueprints/VRPawn` OtherActor)
  (`KismetSystemLibrary.MoveComponentTo` (`self.ButtonRoot`) (- (`self.ButtonStart`) (0.0 5.0 0.0)) (struct) false false 0.1))

(event `self.ReceiveActorEndOverlap`
  (params (OtherActor :type "Actor Object Reference"))
  (cast `/Game/VRTemplate/Blueprints/VRPawn` OtherActor)
  (`KismetSystemLibrary.MoveComponentTo` (`self.ButtonRoot`) (`self.ButtonStart`) (struct) false false 0.1))

(fn `UserConstructionScript`)