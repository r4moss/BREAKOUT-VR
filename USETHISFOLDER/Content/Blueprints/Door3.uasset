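; VR door that swings when a motion controller grabs and moves its grab component.
; Grabbing stores the controller and starts a fast looping timer on UpdateRotation, and dropping clears both.
; Each tick adds the Z difference between the grab component's relative location and the controller's position in that component's space to Door2's yaw, clamped to a symmetric swing limit.
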(event `self.GrabComponent.OnGrabbed`
  (params (`Motion controller` :type "MotionControllerComponent Object Reference"))
  (set `self.Motion Controller` `Motion controller`)
  (bind _returnvalue (`KismetSystemLibrary.K2_SetTimer` null "UpdateRotation" 0.01 true))
  (set `self.Timer` _returnvalue))

(event `self.GrabComponent.OnDropped`
  (`KismetSystemLibrary.K2_ClearAndInvalidateTimerHandle` (`self.Timer`))
  (set `self.Motion Controller` null))

(fn `UpdateRotation`
  (bind _grabcomponent (`self.GrabComponent`))
  (bind _door2 (`self.Door2`))
  (bind (_relativerotation_roll _relativerotation_pitch _relativerotation_yaw) (`KismetMathLibrary.BreakRotator` (`SceneComponent.RelativeRotation` _door2)))
  (bind _returnvalue_location (`KismetMathLibrary.BreakTransform` (`KismetMathLibrary.MakeRelativeTransform` (`SceneComponent.K2_GetComponentToWorld` (`self.Motion Controller`)) (`SceneComponent.K2_GetComponentToWorld` _grabcomponent))))
  (bind (_returnvalue_x _returnvalue_y _returnvalue_z) (`KismetMathLibrary.BreakVector` (- (`SceneComponent.RelativeLocation` _grabcomponent) _returnvalue_location)))
  (`SceneComponent.K2_SetRelativeRotation` _door2 (`KismetMathLibrary.MakeRotator` _relativerotation_roll _relativerotation_pitch (`KismetMathLibrary.FClamp` (+ _relativerotation_yaw _returnvalue_z) -83.0 83.0)) false false))

(fn `UserConstructionScript`)