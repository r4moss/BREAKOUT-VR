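; Timer Blueprint that counts up elapsed minutes and seconds and displays them on a TextRender component.
; Tick runs through a one-second Delay to increment Seconds, rolling over into Minutes at 60.
; The text is rebuilt with FormatText, zero-padding seconds below ten except on rollover and in the initial BeginPlay display.
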(event `self.ReceiveTick`
  (params (DeltaSeconds :type "Float (single-precision)"))
  (`KismetSystemLibrary.Delay` 1.0)
  (bind _result (`/Engine/EditorBlueprintResources/StandardMacros.IncrementInt` (`self.Seconds`))
    (:`  `
      (set `self.Seconds` _result)
      (if (>= (`self.Seconds`) 60)
        (set `self.Seconds` 0)
        (bind _result_2 (`/Engine/EditorBlueprintResources/StandardMacros.IncrementInt` (`self.Minutes`))
          (:`  `
            (set `self.Minutes` _result_2)
            (`TextRenderComponent.K2_SetText` (`self.TextRender`) (`|FormatText` "{Minutes}:{Seconds}" (`self.Minutes`) (`self.Seconds`)) :!label _label)))
        (elif (< (`self.Seconds`) 10)
          (`TextRenderComponent.K2_SetText` (`self.TextRender`) (`|FormatText` "{Minutes}:0{Seconds}" (`self.Minutes`) (`self.Seconds`)))
          (else
            (goto _label)))))))

(event `self.ReceiveBeginPlay`
  (`TextRenderComponent.K2_SetText` (`self.TextRender`) (`|FormatText` "{Minutes}:{Seconds}" (`self.Minutes`) (`self.Seconds`))))

(fn `UserConstructionScript`)