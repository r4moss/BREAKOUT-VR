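; BlackButton is a fusebox button Blueprint that reacts to actors overlapping it.
; On overlap begin it calls the parent handler, then prints its Value to the screen through a DoOnce gate.
; On overlap end it passes the other actor and Value to EndOverlap, then resets the gate for the next overlap.
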(event `self.ReceiveActorBeginOverlap`
  (params (OtherActor :type "Actor Object Reference"))
  (`parent.ReceiveActorBeginOverlap` OtherActor)
  (`/Engine/EditorBlueprintResources/StandardMacros.DoOnce` false :!label _label
    (:`Completed`
      (`KismetSystemLibrary.PrintString` (`KismetStringLibrary.Conv_DoubleToString` (`self.Value`)) true true (struct :`G` 0.66 :`B` 1.0 :`A` 1.0) 10.0))))

(event `self.ReceiveActorEndOverlap`
  (params (OtherActor :type "Actor Object Reference"))
  (`self.EndOverlap` OtherActor (`self.Value`))
  (goto _label :!via `Reset`))

(fn `UserConstructionScript`
  (`parent.UserConstructionScript`))