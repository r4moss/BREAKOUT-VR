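; BlueButton is the blue fusebox button Blueprint, a child actor that reacts to overlaps.
; Begin overlap only forwards to the parent implementation.
; End overlap sets ButtonValue to 4, then calls EndOverlap with the other actor and the Value variable.
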(event `self.ReceiveActorBeginOverlap`
  (params (OtherActor :type "Actor Object Reference"))
  (`parent.ReceiveActorBeginOverlap` OtherActor))

(event `self.ReceiveActorEndOverlap`
  (params (OtherActor :type "Actor Object Reference"))
  (set `self.ButtonValue` 4)
  (`self.EndOverlap` OtherActor (`self.Value`)))

(fn `UserConstructionScript`
  (`parent.UserConstructionScript`))