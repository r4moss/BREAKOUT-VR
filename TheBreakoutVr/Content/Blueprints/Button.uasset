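; A VR push button that visually depresses while the VRPawn overlaps its Box trigger.
; BeginPlay caches the rest location of Cube1, then overlap begin and end events use MoveComponentTo to slide it slightly down and back.
; Only the press animation is implemented; the button triggers no other action.
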(event `self.ReceiveBeginPlay`
  (set `self.ButtonStart` (`SceneComponent.RelativeLocation` (`self.Cube1`))))

(event `self.Box.OnComponentBeginOverlap`
  (params (OverlappedComponent :type "PrimitiveComponent Object Reference") (OtherActor :type "Actor Object Reference") (OtherComp :type "PrimitiveComponent Object Reference") (OtherBodyIndex :type Integer) (bFromSweep :type Boolean) (SweepResult :type "HitResult Structure (by ref)"))
  (cast `/Game/VRTemplate/Blueprints/VRPawn` OtherActor)
  (`KismetSystemLibrary.MoveComponentTo` (`self.Cube1`) (- (`self.ButtonStart`) (0.0 0.0 5.0)) (struct) false false 0.1))

(event `self.Box.OnComponentEndOverlap`
  (params (OverlappedComponent :type "PrimitiveComponent Object Reference") (OtherActor :type "Actor Object Reference") (OtherComp :type "PrimitiveComponent Object Reference") (OtherBodyIndex :type Integer))
  (cast `/Game/VRTemplate/Blueprints/VRPawn` OtherActor)
  (`KismetSystemLibrary.MoveComponentTo` (`self.Cube1`) (`self.ButtonStart`) (struct) false false 0.1))

(fn `UserConstructionScript`)