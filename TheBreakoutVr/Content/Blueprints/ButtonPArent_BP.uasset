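; Parent Blueprint for a pressable VR button that passes input to a Box actor's code calculation.
; When a VRPawn overlaps it, the button mesh slides 5 units along negative Y from its cached start position.
; The custom EndOverlap event slides the mesh back and sends its parameter to CodeCalculate on the Box actor found by class lookup.
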(event `self.ReceiveBeginPlay`
  (set `self.ButtonStart` (`SceneComponent.RelativeLocation` (`self.ButtonStaticMesh`))))

(event `self.ReceiveActorBeginOverlap`
  (params (OtherActor :type "Actor Object Reference"))
  (cast `/Game/VRTemplate/Blueprints/VRPawn` OtherActor)
  (`KismetSystemLibrary.MoveComponentTo` (`self.ButtonStaticMesh`) (- (`self.ButtonStart`) (0.0 5.0 0.0)) (struct :`Roll` 90.0) false false 0.1))

(event `EndOverlap`
  (params (OtherActor :type "Actor Object Reference") (NewParam :type Integer))
  (`KismetSystemLibrary.MoveComponentTo` (`self.ButtonStaticMesh`) (`self.ButtonStart`) (struct :`Roll` 90.0) false false 0.1)
  (bind _returnvalue (`GameplayStatics.GetActorOfClass` "/Game/Blueprints/Box.Box_C"))
  (`/Game/Blueprints/Box.CodeCalculate` _returnvalue NewParam))

(fn `UserConstructionScript`)